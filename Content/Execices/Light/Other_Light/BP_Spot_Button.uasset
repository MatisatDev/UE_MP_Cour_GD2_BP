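; BP_Spot_Button is a light Blueprint that brightens four spot lights when the player character signals its Beginning event.
; On BeginPlay it casts the first player's character to BP_ThirdPersonCharacter and binds TurnONLight to that Beginning dispatcher.
; TurnONLight sets all four spot light components to the same fixed high intensity, with no path to switch them off.
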(event Custom|Turn%20ON%20Light
  (Utilities|FlowControl|Sequence
    (:then_0
      (Rendering|Components|Light|SetIntensity (Variables|Default|GetSpotLight3) 4.1e+04))
    (:then_1
      (Rendering|Components|Light|SetIntensity (Variables|Default|GetSpotLight2) 4.1e+04))
    (:then_2
      (Rendering|Components|Light|SetIntensity (Variables|Default|GetSpotLight1) 4.1e+04))
    (:then_3
      (Rendering|Components|Light|SetIntensity (Variables|Default|GetSpotLight) 4.1e+04))))

(event EventBeginPlay
  (bind _asbp_third_person_character (Utilities|Casting|CastToBP_ThirdPersonCharacter (Game|GetPlayerCharacter 0)))
  (EventDispatchers|BindEventtoBeginning _asbp_third_person_character (delegate Custom|Turn%20ON%20Light)))

(fn ConstructionScript)