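; BP_Win_Light is a light actor that signals victory once the doors are closed.
; On BeginPlay it caches BP_ThirdPersonGameMode, whose AllDoorClose counter TurnONLight? compares to the required total of three.
; When they match, it reveals the first Text3DActor found in the level, raises DorrLight to high intensity and plays demonic laughter and victory sounds.
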(event Custom|Turn%20ON%20Light%20?
  (if (== (Variables|/Game/ThirdPerson/Blueprints/BP_ThirdPersonGameMode.BP_ThirdPersonGameMode_C|GetAll%20Door%20Close%20? (Variables|Default|GetAs%20BP%20Third%20Person%20Game%20Mode)) 3)
    (bind _returnvalue (Actor|GetActorOfClass "/Script/Text3D.Text3DActor"))
    (Rendering|SetVisibility (Variables|/Script/Text3D.Text3DActor|GetText3DComponent _returnvalue) true false)
    (Rendering|Components|Light|SetIntensity (Variables|Default|GetDorrLight) 1e+05)
    (Audio|PlaySound2D "/Game/Sound/Rire_démoniaque.Rire_démoniaque" 1.0 1.0 0.0 0 0)
    (Audio|PlaySound2D "/Game/Sound/Victoire.Victoire" 1.0 1.0 0.0 0 0)))

(event EventBeginPlay
  (bind _asbp_third_person_game_mode (Utilities|Casting|CastToBP_ThirdPersonGameMode (Game|GetGameMode)))
  (Variables|Default|SetAs%20BP%20Third%20Person%20Game%20Mode _asbp_third_person_game_mode))

(fn ConstructionScript)