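; BP_First_Trigger is a one-shot interactable that switches on three trigger actors and a spotlight rig.
; On its first Interact it plays a click sound, then calls the ON events of BP_Trigger_1, BP_Trigger_2 and BP_Trigger_3.
; It then raises the intensity of three spotlights on BP_Spot_Button and sets ButtonPush to block repeat use.
; Each target is found with GetActorOfClass rather than a stored reference.
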(event EventBeginPlay)

(event EventInteract
  (if (not (Variables|Default|GetButton%20push%20?))
    (Audio|PlaySound2D "/Game/Sound/Cool_Click.Cool_Click" 1.0 1.0 0.0 0 0)
    (Utilities|FlowControl|Sequence
      (:then_0
        (bind _returnvalue (Actor|GetActorOfClass "/Game/Execices/Trigger/Other_Trigger/BP_Trigger_1.BP_Trigger_1_C"))
        (Default|TriggerOneON _returnvalue))
      (:then_1
        (bind _returnvalue_2 (Actor|GetActorOfClass "/Game/Execices/Trigger/Other_Trigger/BP_Trigger_2.BP_Trigger_2_C"))
        (Default|TriggerTwoON _returnvalue_2))
      (:then_2
        (bind _returnvalue_3 (Actor|GetActorOfClass "/Game/Execices/Trigger/Other_Trigger/BP_Trigger_3.BP_Trigger_3_C"))
        (Default|TriggerThreeON _returnvalue_3))
      (:then_3
        (bind _returnvalue_4 (Actor|GetActorOfClass "/Game/Execices/Light/Other_Light/BP_Spot_Button.BP_Spot_Button_C"))
        (Utilities|FlowControl|Sequence
          (:then_0
            (Rendering|Components|Light|SetIntensity (Variables|/Game/Execices/Light/Other_Light/BP_Spot_Button.BP_Spot_Button_C|GetSpotLight _returnvalue_4) 4.1e+04))
          (:then_1
            (Rendering|Components|Light|SetIntensity (Variables|/Game/Execices/Light/Other_Light/BP_Spot_Button.BP_Spot_Button_C|GetSpotLight1 _returnvalue_4) 4.1e+04))
          (:then_2
            (Rendering|Components|Light|SetIntensity (Variables|/Game/Execices/Light/Other_Light/BP_Spot_Button.BP_Spot_Button_C|GetSpotLight2 _returnvalue_4) 4.1e+04)
            (Variables|Default|SetButton%20push%20? true)))))))

(fn ConstructionScript)