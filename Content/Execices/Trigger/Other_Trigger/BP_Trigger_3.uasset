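; BP_Trigger_3 is an interactable trigger that opens the three exercise doors when used.
; Interact plays a click sound, then finds BP_DoorExo_1, BP_DoorExo_2 and BP_DoorExo_3 by class and calls DoorOpen on each.
; A separate Trigger_Three_ON event switches the Cube's collision response to Overlap on all channels.
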(event Custom|Trigger_Three_ON
  (Collision|SetCollisionResponsetoAllChannels (Variables|Default|GetCube) "ECR_Overlap"))

(event EventInteract
  (Audio|PlaySound2D "/Game/Sound/Cool_Click.Cool_Click" 1.0 1.0 0.0 0 0)
  (Utilities|FlowControl|Sequence
    (:then_0
      (bind _returnvalue (Actor|GetActorOfClass "/Game/Execices/Door/BP_DoorExo_1.BP_DoorExo_1_C"))
      (Default|DoorOpen _returnvalue))
    (:then_1
      (bind _returnvalue_2 (Actor|GetActorOfClass "/Game/Execices/Door/BP_DoorExo_2.BP_DoorExo_2_C"))
      (Default|DoorOpen _returnvalue_2))
    (:then_2
      (bind _returnvalue_3 (Actor|GetActorOfClass "/Game/Execices/Door/BP_DoorExo_3.BP_DoorExo_3_C"))
      (Default|DoorOpen _returnvalue_3))))

(fn ConstructionScript)