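; BP_Trigger_Restart is an interactable that restarts what appears to be a light-ordering exercise.
; On BeginPlay it caches a reference to BP_ThirdPersonGameMode.
; Interact plays a click sound, then calls CallRestartLight and CallBeginning on the player's BP_ThirdPersonCharacter.
; It then clears the game mode's AllLightsON, StillGood and OrderGood state.
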(event EventBeginPlay
  (bind _asbp_third_person_game_mode (Utilities|Casting|CastToBP_ThirdPersonGameMode (Game|GetGameMode)))
  (Variables|Default|SetAs%20BP%20Third%20Person%20Game%20Mode _asbp_third_person_game_mode))

(event EventInteract
  (bind _as_bp_third_person_game_mode (Variables|Default|GetAs%20BP%20Third%20Person%20Game%20Mode))
  (Audio|PlaySound2D "/Game/Sound/Cool_Click.Cool_Click" 1.0 1.0 0.0 0 0)
  (bind _asbp_third_person_character (Utilities|Casting|CastToBP_ThirdPersonCharacter (Game|GetPlayerCharacter 0)))
  (Default|CallRestartLight _asbp_third_person_character)
  (Default|CallBeginning _asbp_third_person_character)
  (Variables|/Game/ThirdPerson/Blueprints/BP_ThirdPersonGameMode.BP_ThirdPersonGameMode_C|SetAll%20Lights%20ON%20? _as_bp_third_person_game_mode 0)
  (Variables|/Game/ThirdPerson/Blueprints/BP_ThirdPersonGameMode.BP_ThirdPersonGameMode_C|SetStill%20Good _as_bp_third_person_game_mode false)
  (Variables|/Game/ThirdPerson/Blueprints/BP_ThirdPersonGameMode.BP_ThirdPersonGameMode_C|SetOrder%20Good _as_bp_third_person_game_mode false))

(fn ConstructionScript)