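; BP_Door1 is an exercise door Blueprint whose DoorOpen event swings the Porte component open or closed around its yaw axis.
; BeginPlay stores the starting relative rotation, and a Timeline adds its Rotation value to that yaw.
; DoorOpen plays or reverses the Timeline based on PorteFermée, a closed flag recomputed on each update from whether the rotation is below one.
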(event Custom|Door%20Open
  (bind _start_rotation (Variables|Default|GetStart%20Rotation))
  (bind (_roll _pitch _yaw) (Math|Rotator|BreakRotator _start_rotation))
  (if (Variables|Default|GetPorte%20fermée%20?)
    (bind _rotation (Timeline|Timeline Play)
      (:Update
        (Transformation|SetRelativeRotation (Variables|Default|GetPorte) (Math|Rotator|MakeRotator _roll _pitch (+ _rotation _yaw)) false false)
        (Variables|Default|SetPorte%20fermée%20? (< _rotation 1.0))))
    (else
      (Timeline|Timeline Reverse))))

(event EventBeginPlay
  (Variables|Default|SetStart%20Rotation (Variables|/Script/Engine.SceneComponent|GetRelativeRotation (Variables|Default|GetPorte))))

(fn ConstructionScript)