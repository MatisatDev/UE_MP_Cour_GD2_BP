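; BP_DoorEvent is a door that toggles open and closed when an EventLauncher fires its ActivateControlables dispatcher, in an event dispatcher exercise.
; On BeginPlay it binds DoorMove to that dispatcher and stores the starting rotation of the Porte component.
; DoorMove plays or reverses a yaw-offset Timeline based on PorteFermée, which each update recalculates from the current angle.
; It also calls DoorOpen on the BP_Door1 and BP_Door2 actors found by class.
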(event Custom|Door%20move
  (bind _start_rotation (Variables|Default|GetStart%20Rotation))
  (bind (_roll _pitch _yaw) (Math|Rotator|BreakRotator _start_rotation))
  (Utilities|FlowControl|Sequence
    (:then_0
      (bind _returnvalue (Actor|GetActorOfClass "/Game/Exercices/BP_Door1.BP_Door1_C"))
      (Default|DoorOpen _returnvalue))
    (:then_1
      (if (Variables|Default|GetPorte%20fermée%20?)
        (bind _rotation (Timeline|Timeline Play)
          (:Update
            (Transformation|SetRelativeRotation (Variables|Default|GetPorte) (Math|Rotator|MakeRotator _roll _pitch (+ _rotation _yaw)) false false)
            (Variables|Default|SetPorte%20fermée%20? (< _rotation 1.0))))
        (else
          (Timeline|Timeline Reverse))))
    (:then_2
      (bind _returnvalue_2 (Actor|GetActorOfClass "/Game/Exercices/BP_Door2.BP_Door2_C"))
      (Default|DoorOpen _returnvalue_2))))

(event EventBeginPlay
  (Utilities|FlowControl|Sequence
    (:then_0
      (EventDispatchers|BindEventtoActivateControlables (Variables|Default|GetEvent%20Launcher) (delegate Custom|Door%20move)))
    (:then_1
      (Variables|Default|SetStart%20Rotation (Variables|/Script/Engine.SceneComponent|GetRelativeRotation (Variables|Default|GetPorte))))))

(fn ConstructionScript)