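; BP_Door is an interactive door that the player opens and closes, raising or lowering a BP_Light's intensity with it.
; A Box trigger enables the OuverturePorte input while BP_ThirdPersonCharacter overlaps it.
; Each press plays or reverses a Timeline that adds yaw to the door's starting rotation and derives the PorteFermée closed flag from that value.
; The light is found through GetActorOfClass rather than an assigned reference.
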(event OnComponentBeginOverlap(Box)
  (params (OverlappedComponent :type Primitive%20Component%20Object%20Reference) (OtherActor :type Actor%20Object%20Reference) (OtherComp :type Primitive%20Component%20Object%20Reference) (OtherBodyIndex :type Integer) (bFromSweep :type Boolean) (SweepResult :type Hit%20Result%20Structure%20%28by%20ref%29))
  (Utilities|Casting|CastToBP_ThirdPersonCharacter OtherActor)
  (Input|EnableInput (Game|GetPlayerController 0)))

(event OnComponentEndOverlap(Box)
  (params (OverlappedComponent :type Primitive%20Component%20Object%20Reference) (OtherActor :type Actor%20Object%20Reference) (OtherComp :type Primitive%20Component%20Object%20Reference) (OtherBodyIndex :type Integer))
  (Utilities|Casting|CastToBP_ThirdPersonCharacter OtherActor)
  (Input|DisableInput (Game|GetPlayerController 0)))

(event EventBeginPlay
  (Variables|Default|SetStart%20Rotation (Variables|/Script/Engine.SceneComponent|GetRelativeRotation (Variables|Default|GetPorte))))

(event Input|ActionEvents|InputActionOuverturePorte
  (params (Key :type Key%20Structure :default "None"))
  (bind _start_rotation (Variables|Default|GetStart%20Rotation))
  (bind (_roll _pitch _yaw) (Math|Rotator|BreakRotator _start_rotation))
  (:Pressed
    (if (Variables|Default|GetPorte%20fermée%20?)
      (bind _returnvalue (Actor|GetActorOfClass "/Game/Exercices/BP_Light.BP_Light_C"))
      (Default|IntensityUP _returnvalue)
      (bind _rotation (Timeline|Timeline Play)
        (:Update
          (Transformation|SetRelativeRotation (Variables|Default|GetPorte) (Math|Rotator|MakeRotator _roll _pitch (+ _rotation _yaw)) false false)
          (Variables|Default|SetPorte%20fermée%20? (< _rotation 1.0))))
      (else
        (bind _returnvalue_2 (Actor|GetActorOfClass "/Game/Exercices/BP_Light.BP_Light_C"))
        (Default|IntensityDown _returnvalue_2)
        (Timeline|Timeline Reverse)))))

(fn ConstructionScript)