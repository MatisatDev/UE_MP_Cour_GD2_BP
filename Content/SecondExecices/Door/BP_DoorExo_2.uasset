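; Door actor that toggles between open and closed each time DoorOpen fires, using a FlipFlop.
; A timeline plays or reverses to swing the Porte component's yaw relative to its starting rotation, printing the closed-door count during updates.
; Each toggle decrements or increments AllDoorClose on BP_ThirdPersonGameMode.
; When the timeline finishes in either direction, it calls TurnONLight on the BP_Door_Light found in the level.
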(event Custom|Door%20Open
  (bind _start_rotation (Variables|Default|GetStart%20Rotation))
  (bind (_roll _pitch _yaw) (Math|Rotator|BreakRotator _start_rotation))
  (bind _asbp_third_person_game_mode (Utilities|Casting|CastToBP_ThirdPersonGameMode (Game|GetGameMode)))
  (Variables|Default|SetAs%20BP%20Third%20Person%20Game%20Mode _asbp_third_person_game_mode)
  (Utilities|FlowControl|FlipFlop
    (:A
      (Variables|/Game/ThirdPerson/Blueprints/BP_ThirdPersonGameMode.BP_ThirdPersonGameMode_C|SetAll%20Door%20Close%20? (Variables|Default|GetAs%20BP%20Third%20Person%20Game%20Mode) (- (Variables|/Game/ThirdPerson/Blueprints/BP_ThirdPersonGameMode.BP_ThirdPersonGameMode_C|GetAll%20Door%20Close%20? (Variables|Default|GetAs%20BP%20Third%20Person%20Game%20Mode)) 1))
      (bind _rotation (Timeline|Timeline Play)
        (:Update
          (Transformation|SetRelativeRotation (Variables|Default|GetPorte) (Math|Rotator|MakeRotator _roll _pitch (+ _rotation _yaw)) false false)
          (Development|PrintString (Utilities|String|ToString(Integer) (Variables|/Game/ThirdPerson/Blueprints/BP_ThirdPersonGameMode.BP_ThirdPersonGameMode_C|GetAll%20Door%20Close%20? (Variables|Default|GetAs%20BP%20Third%20Person%20Game%20Mode)))))
        (:Finished
          (bind _returnvalue (Actor|GetActorOfClass "/Game/SecondExecices/Light/Door_Light/BP_Door_Light.BP_Door_Light_C"))
          (Default|TurnONLight? _returnvalue))))
    (:B
      (Variables|/Game/ThirdPerson/Blueprints/BP_ThirdPersonGameMode.BP_ThirdPersonGameMode_C|SetAll%20Door%20Close%20? (Variables|Default|GetAs%20BP%20Third%20Person%20Game%20Mode) (+ (Variables|/Game/ThirdPerson/Blueprints/BP_ThirdPersonGameMode.BP_ThirdPersonGameMode_C|GetAll%20Door%20Close%20? (Variables|Default|GetAs%20BP%20Third%20Person%20Game%20Mode)) 1))
      (Timeline|Timeline Reverse))))

(event EventBeginPlay
  (Variables|Default|SetStart%20Rotation (Variables|/Script/Engine.SceneComponent|GetRelativeRotation (Variables|Default|GetPorte))))

(fn ConstructionScript)